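; Surveillance camera actor that keeps its CineCamera aimed at the player pawn every Tick and can take over the player's view.
; Overlap-style Lap and NoLap events play and reverse a timeline that narrows the field of view to zoom in and widens it back.
; SnapToPlayer eases rotation toward the player on a second timeline and raises CheckSnapFinish meanwhile, though Tick never checks that flag.
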(event Custom|NoLap
  (params (OverlappedActor :type Actor%20Object%20Reference) (OtherActor :type Actor%20Object%20Reference))
  ;[1 1 1] Zoom In & Out Event
  (bind _fov_track (Timeline|ZoomTimeline ReverseFromEnd)
    (:Update
      (Camera|SetFieldOfView (Variables|Default|GetCineCamera) (Math|Float|Lerp 9e+01 3e+01 _fov_track)))))

(event Custom|Lap
  (params (OverlappedActor :type Actor%20Object%20Reference) (OtherActor :type Actor%20Object%20Reference))
  ;[1 1 1] Zoom In & Out Event
  (bind _fov_track (Timeline|ZoomTimeline PlayFromStart)
    (:Update
      (Camera|SetFieldOfView (Variables|Default|GetCineCamera) (Math|Float|Lerp 9e+01 3e+01 _fov_track)))))

(event Custom|Surveillance%20camera
  ;[1 1 1] Setting Survelliance Camera as current Camera
  (Game|Player|SetViewTargetwithBlend (Game|GetPlayerController 0) self 0.0 "VTBlend_Linear" 0.0 false)
  (Development|PrintString (Utilities|String|ToString(Float) (Variables|/Script/Engine.CameraComponent|GetFieldOfView (Variables|Default|GetCineCamera)))))

(event Custom|SnapToPlayer
  (bind _cinecamera (Variables|Default|GetCineCamera))
  (bind _fov_track (Timeline|Timeline PlayFromStart)
    (:Update
      (Variables|Default|SetCheckSnapFinish true)
      (Transformation|SetWorldRotation _cinecamera (Math|Rotator|Lerp(Rotator) (Transformation|GetWorldRotation _cinecamera) (Math|Rotator|FindLookatRotation (Transformation|GetWorldLocation (Variables|Default|GetCineCamera)) (Transformation|GetActorLocation (Game|Player|GetPlayerPawn 0))) _fov_track true) false false))
    (:Finished
      (Variables|Default|SetCheckSnapFinish false))))

(event Custom|fkedSurveillance)

(event EventTick
  (params (DeltaSeconds :type Float%20%28single-precision%29))
  (bind _cinecamera (Variables|Default|GetCineCamera))
  ;[1 1 1] Setting Camera Rotation To always face the Character
  (Transformation|SetWorldRotation _cinecamera (Math|Rotator|FindLookatRotation (Transformation|GetWorldLocation _cinecamera) (Transformation|GetActorLocation (Game|Player|GetPlayerPawn 0))) false false))

(fn ConstructionScript)
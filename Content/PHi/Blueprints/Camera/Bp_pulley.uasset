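; Pulley actor in which Cube and Cube1 move vertically in opposite directions when either of two trigger boxes is overlapped.
; Each box plays its own timeline, mirroring which cube goes up or down, and reverses it when the overlap ends.
; Tick spins Cube2, but only the first box enables it, and that box's timeline disables it on finishing.
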(event OnComponentBeginOverlap(Box)
  (params (OverlappedComponent :type Primitive%20Component%20Object%20Reference) (OtherActor :type Actor%20Object%20Reference) (OtherComp :type Primitive%20Component%20Object%20Reference) (OtherBodyIndex :type Integer) (bFromSweep :type Boolean) (SweepResult :type Hit%20Result%20Structure%20%28by%20ref%29))
  (Actor|Tick|SetActorTickEnabled true)
  (bind _newtrack_3 (Timeline|Timeline Play)
    (:Update
      (Transformation|SetRelativeLocation (Variables|Default|GetCube) (Math|Vector|MakeVector 0.0 0.0 (* (.z _newtrack_3) -1.0)) false false)
      (Transformation|SetRelativeLocation (Variables|Default|GetCube1) (Math|Vector|MakeVector 0.0 0.0 (.z _newtrack_3)) false false))
    (:Finished
      (Actor|Tick|SetActorTickEnabled false))))

(event OnComponentEndOverlap(Box)
  (params (OverlappedComponent :type Primitive%20Component%20Object%20Reference) (OtherActor :type Actor%20Object%20Reference) (OtherComp :type Primitive%20Component%20Object%20Reference) (OtherBodyIndex :type Integer))
  (bind _newtrack_3 (Timeline|Timeline Reverse)
    (:Update
      (Transformation|SetRelativeLocation (Variables|Default|GetCube) (Math|Vector|MakeVector 0.0 0.0 (* (.z _newtrack_3) -1.0)) false false)
      (Transformation|SetRelativeLocation (Variables|Default|GetCube1) (Math|Vector|MakeVector 0.0 0.0 (.z _newtrack_3)) false false))
    (:Finished
      (Actor|Tick|SetActorTickEnabled false))))

(event OnComponentBeginOverlap(box1)
  (params (OverlappedComponent :type Primitive%20Component%20Object%20Reference) (OtherActor :type Actor%20Object%20Reference) (OtherComp :type Primitive%20Component%20Object%20Reference) (OtherBodyIndex :type Integer) (bFromSweep :type Boolean) (SweepResult :type Hit%20Result%20Structure%20%28by%20ref%29))
  (bind _newtrack_3 (Timeline|Timeline_0 Play)
    (:Update
      (Transformation|SetRelativeLocation (Variables|Default|GetCube1) (Math|Vector|MakeVector 0.0 0.0 (* (.z _newtrack_3) -1.0)) false false)
      (Transformation|SetRelativeLocation (Variables|Default|GetCube) (Math|Vector|MakeVector 0.0 0.0 (.z _newtrack_3)) false false))))

(event OnComponentEndOverlap(box1)
  (params (OverlappedComponent :type Primitive%20Component%20Object%20Reference) (OtherActor :type Actor%20Object%20Reference) (OtherComp :type Primitive%20Component%20Object%20Reference) (OtherBodyIndex :type Integer))
  (bind _newtrack_3 (Timeline|Timeline_0 Reverse)
    (:Update
      (Transformation|SetRelativeLocation (Variables|Default|GetCube1) (Math|Vector|MakeVector 0.0 0.0 (* (.z _newtrack_3) -1.0)) false false)
      (Transformation|SetRelativeLocation (Variables|Default|GetCube) (Math|Vector|MakeVector 0.0 0.0 (.z _newtrack_3)) false false))))

(event EventBeginPlay
  (Actor|Tick|SetActorTickEnabled false))

(event Collision|EventActorBeginOverlap
  (params (OtherActor :type Actor%20Object%20Reference)))

(event EventTick
  (params (DeltaSeconds :type Float%20%28single-precision%29))
  (Transformation|AddWorldRotation (Variables|Default|GetCube2) "0.000000,0.000000,-10.000000" false false))

(fn ConstructionScript)
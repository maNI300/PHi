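; Spline-bound camera actor that follows the third-person character along the level's BP_Spline.
; SplineStart caches the first BP_Spline, blends the player's view to this actor and looks up the character.
; While the spline is valid, Tick moves SplineCam via VInterpTo, with no interp speed set, to the spline point closest to the character.
; Only the camera's location is driven, not its rotation.
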(event Custom|Spline%20Start
  (bind _returnvalue (Actor|GetActorOfClass "/Game/PHi/Blueprints/Camera/BP_Spline.BP_Spline_C"))
  (Variables|Default|SetSplineRef _returnvalue)
  (Game|Player|SetViewTargetwithBlend (Game|GetPlayerController 0) self 0.0 "VTBlend_Linear" 0.0 false)
  (bind _returnvalue_2 (Actor|GetActorOfClass "/Game/EngineTemplates/ThirdPerson/Blueprints/BP_ThirdPersonCharacter.BP_ThirdPersonCharacter_C")))

(event EventTick
  (params (DeltaSeconds :type Float%20%28single-precision%29))
  (bind _splineref (Variables|Default|GetSplineRef))
  (bind _splinecam (Variables|Default|GetSplineCam))
  (if (Utilities|IsValid _splineref)
    (Transformation|SetWorldLocation _splinecam (Math|Interpolation|VInterpTo (Transformation|GetWorldLocation _splinecam) (Spline|FindLocationClosesttoWorldLocation (Variables|/Game/PHi/Blueprints/Camera/BP_Spline.BP_Spline_C|GetSpline _splineref) (Transformation|GetActorLocation (stale Custom|Spline%20Start _returnvalue_2)) "World") (Utilities|Time|GetWorldDeltaSeconds) 0.0) false false)))

(fn ConstructionScript)
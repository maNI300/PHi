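; Interactable box that the player pushes along its axes, with the character attached to it and its movement disabled.
; On interact, X/Y overlap volumes choose the side to snap to, and camera facing maps input axes to push directions.
; The dominant input axis drives a timeline that moves the box when a box trace finds the path clear.
; It also sets the character's interaction and pushing modes, printing the latter every tick.
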(event Custom|Event_Push
  (params (Push%20Direction%20In%20Axis :type Vector))
  ;[1 1 1] Push Event
  (if (Variables|Default|GetCanUseTimeline)
    (Variables|Default|SetLastActorLocation (Transformation|GetActorLocation))
    (bind _push (Timeline|Push_Timeline PlayFromStart)
      (:Update
        (Variables|Default|SetCanUseTimeline false)
        (Transformation|SetActorRelativeLocation (+ (Variables|Default|GetLastActorLocation) (* _push Push%20Direction%20In%20Axis (Variables|Default|GetPush%20Speed)))))
      (:Finished
        (Variables|Default|SetCanUseTimeline true)))))

(event EventTick
  (params (DeltaSeconds :type Float%20%28single-precision%29))
  (bind _phi_charater_ref (Variables|Default|GetPHI_Charater_Ref)
    (:then
      (Development|PrintString (Utilities|String|EnumtoString (Variables|/Game/PHi/Blueprints/Character/BP_Phi_Character.BP_Phi_Character_C|GetActivePushingMode _phi_charater_ref)) true true "(R=0.007231,G=0.375000,B=0.299823,A=1.000000)" 2.0 "16794"))
    (:else)))

(event EventInteractStarted
  (params (PHI_Character_Ref :type BP%20Phi%20Character%20Object%20Reference))
  ;[1 1 1] Interact_Started
  (Utilities|IsValid PHI_Character_Ref
    (:Is%20Valid
      (Variables|Default|SetPHI_Charater_Ref PHI_Character_Ref)
      ;[1 1 1] Attaching Player To Box  According to Where he overlap
      (if (Collision|IsOverlappingActor (Variables|Default|GetX-AxisCollision) (Variables|Default|GetPHI_Charater_Ref) :!class /Script/Engine.PrimitiveComponent)
        (CallFunction|FaceCharacterTowardsBox (Transformation|GetActorForwardVector))
        (CallFunction|SetPushDirectiononAxis :!label _label)
        (Pawn|Components|CharacterMovement|DisableMovement (Variables|/Script/Engine.Character|GetCharacterMovement (Variables|Default|GetPHI_Charater_Ref)))
        (Transformation|AttachActorToActor (Variables|Default|GetPHI_Charater_Ref) self "None" "KeepWorld" "KeepWorld" "KeepWorld" false)
        (Variables|/Game/PHi/Blueprints/Character/BP_Phi_Character.BP_Phi_Character_C|SetActiveInteractionMode (Variables|Default|GetPHI_Charater_Ref) "NewEnumerator1")
        (elif (Collision|IsOverlappingActor (Variables|Default|GetY-AxisCollision) (Variables|Default|GetPHI_Charater_Ref) :!class /Script/Engine.PrimitiveComponent)
          (CallFunction|FaceCharacterTowardsBox (Transformation|GetActorRightVector))
          (goto _label))))))

(event EventInteractCompleted
  ;[1 1 1] Interact Completed
  (bind _phi_charater_ref (Variables|Default|GetPHI_Charater_Ref)
    (:then
      (Variables|/Script/Engine.CharacterMovementComponent|SetbOrientRotationToMovement (Variables|/Script/Engine.Character|GetCharacterMovement _phi_charater_ref) true)
      (Pawn|Components|CharacterMovement|SetMovementMode (Variables|/Script/Engine.Character|GetCharacterMovement (Variables|Default|GetPHI_Charater_Ref)) "MOVE_Walking" 0)
      (Audio|Components|Audio|Stop (Variables|Default|GetPush_Timeline))
      (Variables|Default|SetCanUseTimeline true)
      (Variables|/Game/PHi/Blueprints/Character/BP_Phi_Character.BP_Phi_Character_C|SetActiveInteractionMode (Variables|Default|GetPHI_Charater_Ref) "NewEnumerator0"))
    (:else)))

(event EventInteractTriggered
  (bind _phi_charater_ref (Variables|Default|GetPHI_Charater_Ref))
  (bind _phi_charater_ref_2 (Variables|Default|GetPHI_Charater_Ref))
  ;[1 1 1] Interact Triggered
  (Variables|Default|GetPHI_Charater_Ref
    (:then
      (if (and (== (Variables|/Game/PHi/Blueprints/Character/BP_Phi_Character.BP_Phi_Character_C|GetForwardAxisValue _phi_charater_ref) 0.0) (== (Variables|/Game/PHi/Blueprints/Character/BP_Phi_Character.BP_Phi_Character_C|GetRightAxisValue _phi_charater_ref) 0.0))
        (Utilities|ResetTimeline)
        (Variables|/Game/PHi/Blueprints/Character/BP_Phi_Character.BP_Phi_Character_C|SetActivePushingMode (Variables|Default|GetPHI_Charater_Ref) "NewEnumerator0")
        (elif (>= (Math|Float|Absolute(Float) (Variables|/Game/PHi/Blueprints/Character/BP_Phi_Character.BP_Phi_Character_C|GetForwardAxisValue _phi_charater_ref_2)) (Math|Float|Absolute(Float) (Variables|/Game/PHi/Blueprints/Character/BP_Phi_Character.BP_Phi_Character_C|GetRightAxisValue _phi_charater_ref_2)))
          (|Forward/BackwardMovement)
          (else
            (|Right/LeftMovement)))))
    (:else)))

(fn ConstructionScript)

(fn FaceCharacterTowardsBox
  (params (Forward/Right%20Vector :type Vector))
  (bind _phi_charater_ref (Variables|Default|GetPHI_Charater_Ref))
  (bind _returnvalue (Transformation|GetActorForwardVector _phi_charater_ref))
  (bind _returnvalue_2 (Math|Vector|DotProduct Forward/Right%20Vector _returnvalue))
  (bind _returnvalue_3 (> _returnvalue_2 0.0))
  (bind _returnvalue_4 (Math|Float|SelectFloat 1.0 -1.0 _returnvalue_3))
  (bind _returnvalue_5 (* Forward/Right%20Vector _returnvalue_4))
  (Variables|/Script/Engine.CharacterMovementComponent|SetbOrientRotationToMovement (Variables|/Script/Engine.Character|GetCharacterMovement (Variables|Default|GetPHI_Charater_Ref)) false)
  (Variables|Default|SetPush%20Direction _returnvalue_5)
  (Transformation|SetActorRotation (Variables|Default|GetPHI_Charater_Ref) (Math|Rotator|MakeRotfromX _returnvalue_5))
  (Transformation|SetActorLocation (Variables|Default|GetPHI_Charater_Ref) (Math|Vector|MakeVector (.x (+ (Transformation|GetActorLocation) (* (Variables|Default|GetPush%20Direction) (* (Variables|Default|GetDistanceFromBox) -1.0)))) (.y (+ (Transformation|GetActorLocation) (* (Variables|Default|GetPush%20Direction) (* (Variables|Default|GetDistanceFromBox) -1.0)))) (.z (Transformation|GetActorLocation (Variables|Default|GetPHI_Charater_Ref)))) false false))

(fn CanPush
  (params (Push_Direction :type Vector))
  (bind _returnvalue (Transformation|GetActorLocation))
  (Variables|Default|GetPHI_Charater_Ref
    (:then
      (bind _returnvalue_2 (Collision|BoxTraceByChannel (+ _returnvalue "0.000000,0.000000,1.000000") (+ _returnvalue (* Push_Direction (Math|Float|SelectFloat 3e+01 3.0 (Utilities|Operators|EqualEqual Push_Direction (Utilities|ChangePushDirectiononAngle 1.8e+02) 0.0))) "0.000000,0.000000,1.000000") (/ (.boxextent (StaticMesh|GetBounds (Variables|/Script/Engine.StaticMeshComponent|GetStaticMesh (Variables|Default|GetCube)))) 2.0) "0, 0, 0" "TraceTypeQuery1" false (Utilities|Array|MakeArray (Variables|Default|GetPHI_Charater_Ref)) "ForOneFrame"))
      (if _returnvalue_2
        (return false)
        (else
          (return true))))
    (:else)))

(fn SetPushDirectiononAxis
  (bind _push_direction (Variables|Default|GetPush%20Direction))
  (if (and (< (Math|Vector|DotProduct (Transformation|GetActorForwardVector (Game|GetPlayerCameraManager 0)) _push_direction) 0.0) (< (Math|Vector|DotProduct (Transformation|GetActorRightVector (Game|GetPlayerCameraManager 0)) _push_direction) 0.0))
    (Variables|Default|SetPushDirectionForwardAxis (Utilities|ChangePushDirectiononAngle 1.8e+02))
    (Variables|Default|SetPushDirectionBackwardAxis (Variables|Default|GetPush%20Direction))
    (Variables|Default|SetPushDirectionRightAxis (Utilities|ChangePushDirectiononAngle 2.7e+02))
    (Variables|Default|SetPushDirectionLeftAxis (Utilities|ChangePushDirectiononAngle 9e+01))
    (elif (< (Math|Vector|DotProduct (Transformation|GetActorRightVector (Game|GetPlayerCameraManager 0)) (Variables|Default|GetPush%20Direction)) 0.0)
      (Variables|Default|SetPushDirectionForwardAxis (Utilities|ChangePushDirectiononAngle 9e+01))
      (Variables|Default|SetPushDirectionBackwardAxis (Utilities|ChangePushDirectiononAngle 2.7e+02))
      (Variables|Default|SetPushDirectionRightAxis (Utilities|ChangePushDirectiononAngle 1.8e+02))
      (Variables|Default|SetPushDirectionLeftAxis (Variables|Default|GetPush%20Direction))
      (elif (< (Math|Vector|DotProduct (Transformation|GetActorForwardVector (Game|GetPlayerCameraManager 0)) (Variables|Default|GetPush%20Direction)) 0.0)
        (Variables|Default|SetPushDirectionForwardAxis (Utilities|ChangePushDirectiononAngle 2.7e+02))
        (Variables|Default|SetPushDirectionBackwardAxis (Utilities|ChangePushDirectiononAngle 9e+01))
        (Variables|Default|SetPushDirectionRightAxis (Variables|Default|GetPush%20Direction))
        (Variables|Default|SetPushDirectionLeftAxis (Utilities|ChangePushDirectiononAngle 1.8e+02))
        (else
          (Variables|Default|SetPushDirectionForwardAxis (Variables|Default|GetPush%20Direction))
          (Variables|Default|SetPushDirectionBackwardAxis (Utilities|ChangePushDirectiononAngle 1.8e+02))
          (Variables|Default|SetPushDirectionRightAxis (Utilities|ChangePushDirectiononAngle 9e+01))
          (Variables|Default|SetPushDirectionLeftAxis (Utilities|ChangePushDirectiononAngle 2.7e+02)))))))

(fn SetPushState
  (params (Push%20DIrection%20Axis :type Vector))
  (if (Utilities|Operators|EqualEqual Push%20DIrection%20Axis (Variables|Default|GetPush%20Direction) 0.0)
    (Variables|/Game/PHi/Blueprints/Character/BP_Phi_Character.BP_Phi_Character_C|SetActivePushingMode (Variables|Default|GetPHI_Charater_Ref) "NewEnumerator1")
    (elif (Utilities|Operators|EqualEqual Push%20DIrection%20Axis (Utilities|ChangePushDirectiononAngle 1.8e+02) 0.0)
      (Variables|/Game/PHi/Blueprints/Character/BP_Phi_Character.BP_Phi_Character_C|SetActivePushingMode (Variables|Default|GetPHI_Charater_Ref) "NewEnumerator2")
      (elif (Utilities|Operators|EqualEqual Push%20DIrection%20Axis (Utilities|ChangePushDirectiononAngle 9e+01) 0.0)
        (Variables|/Game/PHi/Blueprints/Character/BP_Phi_Character.BP_Phi_Character_C|SetActivePushingMode (Variables|Default|GetPHI_Charater_Ref) "NewEnumerator3")
        (elif (Utilities|Operators|EqualEqual Push%20DIrection%20Axis (Utilities|ChangePushDirectiononAngle 2.7e+02) 0.0)
          (Variables|/Game/PHi/Blueprints/Character/BP_Phi_Character.BP_Phi_Character_C|SetActivePushingMode (Variables|Default|GetPHI_Charater_Ref) "NewEnumerator4"))))))

(event Custom|Reset%20Right%20Do%20Once
  (Utilities|FlowControl|DoOnce false) ; enters at Reset
)

(event Custom|Reset%20Left%20Do%20Once
  (Utilities|FlowControl|DoOnce false) ; enters at Reset
)

(event Custom|Reset%20Forward%20Do%20Once
  (Utilities|FlowControl|DoOnce false) ; enters at Reset
)

(event Custom|Reset%20Backward%20Do%20Once
  (Utilities|FlowControl|DoOnce false) ; enters at Reset
)
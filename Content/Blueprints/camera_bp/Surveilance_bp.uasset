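; Surveillance camera actor that tracks the player pawn and can take over the player's view.
; The Surveillancecamera event sets this actor as the first player controller's view target.
; Tick turns the CineCamera toward the pawn with a look-at rotation.
; Overlap handlers Lap and NoLap use separate timelines to lerp the field of view, zooming in and back out, without filtering the overlapping actor.
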(event Custom|NoLap
  (params (OverlappedActor :type Actor%20Object%20Reference) (OtherActor :type Actor%20Object%20Reference))
  (bind _newtrack_0 (Timeline|Timeline_0 PlayFromStart)
    (:Update
      (Camera|SetFieldOfView (Variables|Default|GetCineCamera) (Math|Float|Lerp 3e+01 9e+01 _newtrack_0)))))

(event Custom|Lap
  (params (OverlappedActor :type Actor%20Object%20Reference) (OtherActor :type Actor%20Object%20Reference))
  (bind _newtrack_0 (Timeline|Timeline PlayFromStart)
    (:Update
      (Camera|SetFieldOfView (Variables|Default|GetCineCamera) (Math|Float|Lerp 9e+01 3e+01 _newtrack_0)))))

(event Custom|Surveillance%20camera
  (Game|Player|SetViewTargetwithBlend (Game|GetPlayerController 0) self 0.0 "VTBlend_Linear" 0.0 false))

(event EventTick
  (params (DeltaSeconds :type Float%20%28single-precision%29))
  (bind _cinecamera (Variables|Default|GetCineCamera))
  (Transformation|SetWorldRotation _cinecamera (Math|Rotator|FindLookatRotation (Transformation|GetWorldLocation _cinecamera) (Transformation|GetActorLocation (Game|Player|GetPlayerPawn 0))) false false))

(fn ConstructionScript)
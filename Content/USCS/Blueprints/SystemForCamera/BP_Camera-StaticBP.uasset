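; Zone-triggered static camera for the USCS camera system that takes over the view with a blend when the player enters its influencer volume.
; Entry optionally triggers a fade and notifies the other camera Blueprints, with DoOnce gates and short delays arbitrating handoffs between overlapping zones and on exit.
; Tick can track the player with clamped, interpolated look-at rotation, plus optional input-driven yaw and pitch offsets.
; The construction script selects the billboard sprite.
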(event OnComponentBeginOverlap(StaticCameraZoneInfluencer)
  (params (OverlappedComponent :type Primitive%20Component%20Object%20Reference) (OtherActor :type Actor%20Object%20Reference) (OtherComp :type Primitive%20Component%20Object%20Reference) (OtherBodyIndex :type Integer) (bFromSweep :type Boolean) (SweepResult :type Hit%20Result%20Structure%20%28by%20ref%29))
  (Utilities|IsPlayerCharacter/Pawn? OtherActor
    (:true
      (Utilities|FlowControl|DoOnce false
        (:Completed
          (if (Variables|PARAMETRS:FadeIn:|GetUseFadeIn)
            (if (Variables|Default|GetEventBeginPlay?)
              (Actor|Tick|SetActorTickEnabled true :!label _label)
              (Variables|Default|SetIsOveralpingUscsBP false)
              (for _array_element (Variables|Default|GetCamera-CharacterBP_Ref)
                (Default|BacktoCamera-StaticBP _array_element)
                (for _array_element_2 (Variables|Default|GetUscsForCameraBP_Ref)
                  (Default|BacktoCamera-StaticBP _array_element_2)
                  (for _array_element_3 (Variables|Default|GetCameraBP_Ref)
                    (Default|BacktoCamera-StaticBP _array_element_3))))
              (else
                (for _array_element_4 (Variables|Default|GetCameraBP_Ref)
                  (bind _bc_fadeincamerabp (CallFunction|BCFadeinCameraParameters _array_element_4 (Variables|PARAMETRS:FadeIn:|GetUseFadeIn) (Variables|PARAMETRS:FadeIn:|GetDisable%20Player%20Input%20Controller) (Variables|PARAMETRS:FadeIn:|GetPre%20Fade%20Time) (Variables|PARAMETRS:FadeIn:|GetPre%20Fade%20Color) (Variables|PARAMETRS:FadeIn:|GetPre%20Fade%20Should%20Fade%20Audio) (Variables|PARAMETRS:FadeIn:|GetFade%20Time) (Variables|PARAMETRS:FadeIn:|GetFade%20Color) (Variables|PARAMETRS:FadeIn:|GetFade%20from%20Alpha%28X%29%20to%20Alpha%28Y%29) (Variables|PARAMETRS:FadeIn:|GetShould%20Fade%20Audio?) (Variables|PARAMETRS:FadeIn:|GetHold%20When%20Finished?)))
                  (Default|BCFadeinSetting _bc_fadeincamerabp)
                  (goto _label))))
            (else
              (goto _label))))))))

(event OnComponentEndOverlap(StaticCameraZoneInfluencer)
  (params (OverlappedComponent :type Primitive%20Component%20Object%20Reference) (OtherActor :type Actor%20Object%20Reference) (OtherComp :type Primitive%20Component%20Object%20Reference) (OtherBodyIndex :type Integer))
  (Utilities|IsPlayerCharacter/Pawn? OtherActor
    (:true
      (Utilities|FlowControl|Sequence
        (:then_0
          (Utilities|FlowControl|DoOnce false) ; enters at Reset
        )
        (:then_1
          (for _array_element (Variables|Default|GetUscsForCameraBP_Ref)
            (Variables|/Game/USCS/Blueprints/SystemForCamera/BP_USCS_ForCameraBP.BP_USCS_ForCameraBP_C|SetPreviousZoneInfluWasA_UscsZoneInflu _array_element false)
            (Utilities|FlowControl|DoOnce false) ; enters at Reset
          ))))))

(event EventTick
  (params (DeltaSeconds :type Float%20%28single-precision%29))
  (bind _returnvalue (CallFunction|GetPlayerType(PawnorCharacter)))
  (bind _returnvalue_2 (Input|EnhancedActionValues|GetIA_RotateCamera))
  (bind _clampslopel_r (Variables|PARAMETERS:|GetClampSlopeL/R))
  (bind _clampangledown_up (Variables|PARAMETERS:|GetClampAngleDown/Up))
  (bind _clampanglel_r (Variables|PARAMETERS:|GetClampAngleL/R))
  (bind _staticcamera (Variables|Default|GetStaticCamera))
  (bind _angleminv_ (Variables|PARAMETERS:SceneCameraController:|GetAngleMinV:))
  (bind _anglemaxv_ (Variables|PARAMETERS:SceneCameraController:|GetAngleMaxV:))
  (bind _angleminh (Variables|PARAMETERS:SceneCameraController:|GetAngleMinH))
  (bind _anglemaxh (Variables|PARAMETERS:SceneCameraController:|GetAngleMaxH))
  (bind _returnvalue_3 (Transformation|GetActorLocation _returnvalue))
  (bind _returnvalue_4 (/ _anglemaxv_ 3.6e+02))
  (bind _returnvalue_5 (/ _angleminv_ 3.6e+02))
  (bind _returnvalue_6 (/ _angleminh 3.6e+02))
  (bind _returnvalue_7 (/ _anglemaxh 3.6e+02))
  (bind _returnvalue_8 (Transformation|GetWorldLocation _staticcamera))
  (bind _returnvalue_9 (Math|Float|Clamp(Float) (.x _returnvalue_2) _returnvalue_6 _returnvalue_7))
  (bind _returnvalue_10 (Math|Rotator|FindLookatRotation _returnvalue_8 _returnvalue_3))
  (bind _returnvalue_11 (Math|Float|Clamp(Float) (.y _returnvalue_2) _returnvalue_5 _returnvalue_4))
  (bind _returnvalue_12 (* 360 _returnvalue_9))
  (bind _returnvalue_13 (* -3600 _returnvalue_9))
  (bind _returnvalue_14 (* -360 _returnvalue_11))
  (bind _returnvalue_15 (* 360 _returnvalue_11))
  (Utilities|FlowControl|Sequence
    (:then_0
      (if (Variables|PARAMETERS:|GetTrackingPlayer)
        (Transformation|SetWorldRotation _staticcamera (Math|Interpolation|RInterpTo (Transformation|GetWorldRotation _staticcamera) (Math|Rotator|MakeRotator (Math|Float|Clamp(Float) (.roll _returnvalue_10) (.x _clampslopel_r) (.y _clampslopel_r)) (- (Math|Float|Clamp(Float) (.pitch _returnvalue_10) (.x _clampangledown_up) (.y _clampangledown_up)) (Variables|Default|GetRotateCameraV)) (+ (Math|Float|Clamp(Float) (.yaw _returnvalue_10) (.x _clampanglel_r) (.y _clampanglel_r)) (Variables|Default|GetRotateCameraH))) (Utilities|Time|GetWorldDeltaSeconds) (Variables|PARAMETERS:|GetInterpSpeedRotation)) false false))
      (if (Variables|Default|GetIsOveralpingUscsBP)
        (Utilities|FlowControl|Sequence
          (:then_0
            (Utilities|FlowControl|DoOnce false :!label _label
              (:Completed
                (Actor|Tick|SetActorTickEnabled false)
                (Utilities|FlowControl|Delay 0.01)
                (CallFunction|EnableControllerInput false self)
                (Variables|Default|SetIsOveralpingUscsBP false)
                (Utilities|FlowControl|DoOnce false
                  (:Completed
                    (for _array_element (Variables|Default|GetUscsForCameraBP_Ref)
                      (Variables|/Game/USCS/Blueprints/SystemForCamera/BP_USCS_ForCameraBP.BP_USCS_ForCameraBP_C|SetPreviousZoneInfluWasA_UscsZoneInflu _array_element true)
                      (for _array_element_2 (Variables|Default|GetCameraBP_Ref)
                        (Default|BacktoCameraBP _array_element_2))))))))
          (:then_1
            (Utilities|FlowControl|Delay 0.01 :!label _label_2)
            (goto _label_3 Reset)))
        (else
          (Utilities|FlowControl|Sequence
            (:then_0
              (if (Collision|IsOverlappingActor (Variables|Default|GetStaticCameraZoneInfluencer) (CallFunction|GetPlayerType(PawnorCharacter)) :!class /Script/Engine.PrimitiveComponent)
                (Utilities|FlowControl|DoOnce false :!label _label_3
                  (:Completed
                    (Game|Player|SetViewTargetwithBlend (Game|GetPlayerController 0) self (Variables|PARAMETERS:|GetBlend:TimeFromOtherCamera) (Variables|PARAMETERS:|GetBlend:Function) (Variables|PARAMETERS:|GetBlend:CurveShape) (Variables|PARAMETERS:|GetBlend:Lock%20Outgoing))))
                (else
                  (goto _label_2))))
            (:then_1
              (Utilities|FlowControl|Delay 0.01)
              (goto _label Reset))))))
    (:then_1
      (Utilities|FlowControl|Sequence
        (:then_0
          (if (Variables|PARAMETERS:SceneCameraController:|GetCanControlCameraRotationH?)
            (if (Variables|PARAMETERS:SceneCameraController:|GetReverseControllerAxisH?)
              (if (== (Variables|PARAMETERS:|GetInterpSpeedRotation) 0.0)
                (Variables|Default|SetRotateCameraH (Math|Interpolation|FInterpTo (Variables|Default|GetRotateCameraH) _returnvalue_13 (Utilities|Time|GetWorldDeltaSeconds) (Variables|PARAMETERS:SceneCameraController:|GetSmoothControllerRotation)))
                (else
                  (Variables|Default|SetRotateCameraH _returnvalue_13)))
              (elif (== (Variables|PARAMETERS:|GetInterpSpeedRotation) 0.0)
                (Variables|Default|SetRotateCameraH (Math|Interpolation|FInterpTo (Variables|Default|GetRotateCameraH) _returnvalue_12 (Utilities|Time|GetWorldDeltaSeconds) (Variables|PARAMETERS:SceneCameraController:|GetSmoothControllerRotation)))
                (else
                  (Variables|Default|SetRotateCameraH _returnvalue_12))))))
        (:then_1
          (if (Variables|PARAMETERS:SceneCameraController:|GetCanControlCameraRotationV?)
            (if (Variables|PARAMETERS:SceneCameraController:|GetReverseControllerAxisV?)
              (if (== (Variables|PARAMETERS:|GetInterpSpeedRotation) 0.0)
                (Variables|Default|SetRotateCameraV (Math|Interpolation|FInterpTo (Variables|Default|GetRotateCameraV) _returnvalue_14 (Utilities|Time|GetWorldDeltaSeconds) (Variables|PARAMETERS:SceneCameraController:|GetSmoothControllerRotation)))
                (else
                  (Variables|Default|SetRotateCameraV _returnvalue_14)))
              (elif (== (Variables|PARAMETERS:|GetInterpSpeedRotation) 0.0)
                (Variables|Default|SetRotateCameraV (Math|Interpolation|FInterpTo (Variables|Default|GetRotateCameraV) _returnvalue_15 (Utilities|Time|GetWorldDeltaSeconds) (Variables|PARAMETERS:SceneCameraController:|GetSmoothControllerRotation)))
                (else
                  (Variables|Default|SetRotateCameraV _returnvalue_15))))))))))

(event EventBeginPlay
  (bind _staticcamera (Variables|Default|GetStaticCamera))
  (Variables|Default|SetEventBeginPlay? true)
  (Variables|Default|SetInitialRotation (Transformation|GetWorldRotation _staticcamera))
  (Variables|Default|SetInitialLocation (Transformation|GetWorldLocation _staticcamera))
  (bind _outactors (Actor|GetAllActorsOfClass "/Game/USCS/Blueprints/SystemForCamera/BP_CameraBP.BP_CameraBP_C"))
  (Variables|Default|SetCameraBP_Ref _outactors)
  (bind _outactors_2 (Actor|GetAllActorsOfClass "/Game/USCS/Blueprints/SystemForCamera/BP_Camera-CharacterBP.BP_Camera-CharacterBP_C"))
  (Variables|Default|SetCamera-CharacterBP_Ref _outactors_2)
  (bind _outactors_3 (Actor|GetAllActorsOfClass "/Game/USCS/Blueprints/SystemForCamera/BP_USCS_ForCameraBP.BP_USCS_ForCameraBP_C"))
  (Variables|Default|SetUscsForCameraBP_Ref _outactors_3)
  (Utilities|FlowControl|Sequence
    (:then_0
      (for _array_element (Variables|Default|GetCameraBP_Ref)
        (Utilities|FlowControl|Delay (+ (Variables|/Game/USCS/Blueprints/DataLibrary/BC_FadeIn.BC_FadeIn_C|GetFadeTime (Variables|/Game/USCS/Blueprints/SystemForCamera/BP_CameraBP.BP_CameraBP_C|GetBC_FadeInCameraBP _array_element)) (Variables|/Game/USCS/Blueprints/DataLibrary/BC_FadeIn.BC_FadeIn_C|GetPreFadeTime (Variables|/Game/USCS/Blueprints/SystemForCamera/BP_CameraBP.BP_CameraBP_C|GetBC_FadeInCameraBP _array_element))))
        (Variables|Default|SetEventBeginPlay? false)))
    (:then_1
      (Variables|Default|SetIsOveralpingUscsBP false)
      (Utilities|FlowControl|Delay 0.01)
      (if (Collision|IsOverlappingActor (Variables|Default|GetStaticCameraZoneInfluencer) (CallFunction|GetPlayerType(PawnorCharacter)) :!class /Script/Engine.PrimitiveComponent)
        (Utilities|FlowControl|DoOnce false
          (:Completed
            (if (Variables|PARAMETRS:FadeIn:|GetUseFadeIn)
              (if (Variables|Default|GetEventBeginPlay?)
                (Actor|Tick|SetActorTickEnabled true :!label _label)
                (Variables|Default|SetIsOveralpingUscsBP false)
                (for _array_element_2 (Variables|Default|GetCamera-CharacterBP_Ref)
                  (Default|BacktoCamera-StaticBP _array_element_2)
                  (for _array_element_3 (Variables|Default|GetUscsForCameraBP_Ref)
                    (Default|BacktoCamera-StaticBP _array_element_3)
                    (for _array_element_4 (Variables|Default|GetCameraBP_Ref)
                      (Default|BacktoCamera-StaticBP _array_element_4))))
                (else
                  (for _array_element_5 (Variables|Default|GetCameraBP_Ref)
                    (bind _bc_fadeincamerabp (CallFunction|BCFadeinCameraParameters _array_element_5 (Variables|PARAMETRS:FadeIn:|GetUseFadeIn) (Variables|PARAMETRS:FadeIn:|GetDisable%20Player%20Input%20Controller) (Variables|PARAMETRS:FadeIn:|GetPre%20Fade%20Time) (Variables|PARAMETRS:FadeIn:|GetPre%20Fade%20Color) (Variables|PARAMETRS:FadeIn:|GetPre%20Fade%20Should%20Fade%20Audio) (Variables|PARAMETRS:FadeIn:|GetFade%20Time) (Variables|PARAMETRS:FadeIn:|GetFade%20Color) (Variables|PARAMETRS:FadeIn:|GetFade%20from%20Alpha%28X%29%20to%20Alpha%28Y%29) (Variables|PARAMETRS:FadeIn:|GetShould%20Fade%20Audio?) (Variables|PARAMETRS:FadeIn:|GetHold%20When%20Finished?)))
                    (Default|BCFadeinSetting _bc_fadeincamerabp)
                    (goto _label))))
              (else
                (goto _label)))))))))

(event EventBacktoCamera-CharacterBP
  (Actor|Tick|SetActorTickEnabled false)
  (Utilities|FlowControl|Sequence
    (:then_0
      (Utilities|FlowControl|DoOnce false) ; enters at Reset
    )
    (:then_1
      (Utilities|FlowControl|Delay 0.01)
      (Utilities|FlowControl|DoOnce false) ; enters at Reset
    )))

(event EventOnBecomeViewTarget
  (params (PC :type Player%20Controller%20Object%20Reference))
  (Transformation|SetWorldLocationAndRotation (Variables|Default|GetStaticCamera) (Variables|Default|GetInitialLocation) (Variables|Default|GetInitialRotation) false false)
  (CallFunction|EnableControllerInput true self))

(event EventBacktoUscs
  (Variables|Default|SetIsOveralpingUscsBP true))

(event EventOnEndViewTarget
  (params (PC :type Player%20Controller%20Object%20Reference))
  (Actor|Tick|SetActorTickEnabled false)
  (Utilities|FlowControl|Sequence
    (:then_0
      (Utilities|FlowControl|DoOnce false) ; enters at Reset
    )
    (:then_1
      (Utilities|FlowControl|Delay 0.01)
      (Utilities|FlowControl|DoOnce false) ; enters at Reset
    )))

(fn ConstructionScript
  (bind _spritecollection (Variables|Default|GetSpriteCollection))
  (Variables|PARAMETERS:|SetThumnailSelector: (Math|Integer|Clamp(Integer) (Variables|PARAMETERS:|GetThumnailSelector:) 0 (- (Utilities|Array|Length _spritecollection) 1)))
  (Variables|/Script/Engine.BillboardComponent|SetSprite (Variables|Default|GetBillboard) (Utilities|Array|Get(acopy) _spritecollection (Math|Integer|Clamp(Integer) (Variables|PARAMETERS:|GetThumnailSelector:) 0 (- (Utilities|Array|Length _spritecollection) 1)))))